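; Slot-based inventory Blueprint that stores item classes with amounts and creates its main UI widget on BeginPlay.
; AddItem fills partial stacks or empty slots, recursing on overflow and returning any remainder.
; Remove, swap, merge and split functions edit the slot array, generally refreshing affected slot widgets.
; Using an item spawns its class and calls its used event; other helpers toggle visibility and sort descriptions into weapon and item lists.
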(event Custom|UpdateSlotAtIndex
  (params (Index :type Integer))
  ;[1 1 1] Inventory Slot Updater
  (Default|UpdateSlot (Utilities|Array|Get(acopy) (Variables|/Game/Inventory_v2/Inventory_Widgets/Inventory_v2_Widget.Inventory_v2_Widget_C|GetSlot_Widget (Variables|Default|GetInventory_v2_Widget)) Index)))

(event Custom|UseItemAtIndex
  (params (Index :type Integer))
  (bind _slots (Variables|Default|GetSlots))
  (bind _output (Utilities|Array|Get(acopy) _slots Index))
  (bind _itemclass (Utilities|Struct|BreakFInventorySlotStruct _output))
  ;[1 1 1] Use Item
  (if (Utilities|IsValidClass _itemclass)
    (bind _returnvalue (Game|SpawnActorfromClass _itemclass (Math|Transform|MakeTransform "0, 0, 0" "0, 0, 0" "1.000000,1.000000,1.000000") "AlwaysSpawn" "MultiplyWithRoot" 0 self Index 0))
    (Default|EventonUsed _returnvalue)))

(event EventBeginPlay
  (Utilities|Array|Resize (Variables|Default|GetSlots) (Variables|Default|GetAmount_of_Slots))
  (bind _returnvalue (UserInterface|CreateWidget "/Game/Inventory_v2/Inventory_Widgets/Main_Widget.Main_Widget_C" 0 self (Variables|Default|GetSlots_Per_Row)))
  (bind _output_get (Variables|Default|SetMain_Widget _returnvalue))
  (Variables|Default|SetInventory_v2_Widget (Variables|/Game/Inventory_v2/Inventory_Widgets/Main_Widget.Main_Widget_C|GetInventory_Widget _output_get))
  (UserInterface|Viewport|AddtoViewport (Variables|Default|GetMain_Widget) 0))

(fn ConstructionScript)

(fn IsSlotEmpty?
  (params (Index :type Integer))
  (return (not (Utilities|IsValidClass (.ItemClass (Utilities|Struct|BreakFInventorySlotStruct (Utilities|Array|Get(acopy) (Variables|Default|GetSlots) Index)))))))

(fn GetItemInfoatIndex
  (params (Index :type Integer))
  (bind _slots (Variables|Default|GetSlots))
  (bind _output (Utilities|Array|Get(acopy) _slots Index))
  (bind (_itemclass _amount) (Utilities|Struct|BreakFInventorySlotStruct _output))
  (if (Utilities|IsValidClass _itemclass)
    (return false (.Item_Info (Utilities|GetClassDefaults _itemclass)) _amount)
    (else
      (return true "" 0))))

(fn SearchEmptySlot
  (bind (_array_element _array_index) (Utilities|Array|ForEachLoopwithBreak (Variables|Default|GetSlots) :!label _label)
    (:LoopBody
      (if (Utilities|IsValidClass (.ItemClass (Utilities|Struct|BreakFInventorySlotStruct _array_element)))
        ;[1 1 1] Recommendation from #003 top comment
        (LocalVariables|SetLocal_Bool false)
        (else
          (LocalVariables|SetLocal_Bool true)
          (LocalVariables|SetLocal_Index _array_index)
          (goto _label Break))))
    (:Completed
      (return (LocalVariables|GetLocal_Bool) (LocalVariables|GetLocal_Index)))))

(fn SearchFreeStack
  (params (Item_Class :type BP%20Master%20Item%20Class%20Reference))
  (bind (_array_element _array_index) (Utilities|Array|ForEachLoopwithBreak (Variables|Default|GetSlots) :!label _label)
    (:LoopBody
      (if (Utilities|IsValidClass (.ItemClass (Utilities|Struct|BreakFInventorySlotStruct _array_element)))
        (if (and (== (.ItemClass (Utilities|Struct|BreakFInventorySlotStruct _array_element)) Item_Class) (< (.Amount (Utilities|Struct|BreakFInventorySlotStruct _array_element)) (Variables|Default|GetMax_Stack_Size)))
          (LocalVariables|SetLocal_Bool true)
          (LocalVariables|SetLocal_Index _array_index)
          (goto _label Break))))
    (:Completed
      (return (LocalVariables|GetLocal_Bool) (LocalVariables|GetLocal_Index)))))

(fn AddItem
  (params (Item_Class :type BP%20Master%20Item%20Class%20Reference) (Amount :type Integer))
  (LocalVariables|SetLocal_Class Item_Class)
  (LocalVariables|SetLocal_Amount Amount)
  (if (.CanBeStacked (Utilities|Struct|BreakFItemStruct (.Item_Info (Utilities|GetClassDefaults Item_Class))))
    (bind (_success_ _index) (CallFunction|SearchFreeStack (LocalVariables|GetLocal_Class)))
    (if _success_
      (LocalVariables|SetFound_Index _index)
      (if (> (+ (.Amount (Utilities|Struct|BreakFInventorySlotStruct (Utilities|Array|Get(acopy) (Variables|Default|GetSlots) (LocalVariables|GetFound_Index)))) (LocalVariables|GetLocal_Amount)) (Variables|Default|GetMax_Stack_Size))
        (LocalVariables|SetLocal_Amount (- (+ (.Amount (Utilities|Struct|BreakFInventorySlotStruct (Utilities|Array|Get(acopy) (Variables|Default|GetSlots) (LocalVariables|GetFound_Index)))) (LocalVariables|GetLocal_Amount)) (Variables|Default|GetMax_Stack_Size)))
        (Utilities|Array|SetArrayElem (Variables|Default|GetSlots) (LocalVariables|GetFound_Index) (Utilities|Struct|MakeFInventorySlotStruct (LocalVariables|GetLocal_Class) (Variables|Default|GetMax_Stack_Size)))
        (CallFunction|UpdateSlotatIndex (LocalVariables|GetFound_Index))
        (bind _rest (CallFunction|AddItem (LocalVariables|GetLocal_Class) (LocalVariables|GetLocal_Amount)))
        (return true _rest)
        (else
          (Utilities|Array|SetArrayElem (Variables|Default|GetSlots) (LocalVariables|GetFound_Index) (Utilities|Struct|MakeFInventorySlotStruct (LocalVariables|GetLocal_Class) (+ (.Amount (Utilities|Struct|BreakFInventorySlotStruct (Utilities|Array|Get(acopy) (Variables|Default|GetSlots) (LocalVariables|GetFound_Index)))) (LocalVariables|GetLocal_Amount))))
          (CallFunction|UpdateSlotatIndex (LocalVariables|GetFound_Index))
          (return true 0)))
      (else
        (bind (_success__2 _index_2) (CallFunction|SearchEmptySlot))
        (if _success__2
          (bind _output_get (LocalVariables|SetFound_Index _index_2))
          (if (> (LocalVariables|GetLocal_Amount) (Variables|Default|GetMax_Stack_Size))
            (Utilities|Array|SetArrayElem (Variables|Default|GetSlots) _output_get (Utilities|Struct|MakeFInventorySlotStruct (LocalVariables|GetLocal_Class) (Variables|Default|GetMax_Stack_Size)))
            (CallFunction|UpdateSlotatIndex (LocalVariables|GetFound_Index))
            (bind _rest_2 (CallFunction|AddItem (LocalVariables|GetLocal_Class) (- (LocalVariables|GetLocal_Amount) (Variables|Default|GetMax_Stack_Size))))
            (return true _rest_2)
            (else
              (Utilities|Array|SetArrayElem (Variables|Default|GetSlots) (LocalVariables|GetFound_Index) (Utilities|Struct|MakeFInventorySlotStruct (LocalVariables|GetLocal_Class) (LocalVariables|GetLocal_Amount)))
              (CallFunction|UpdateSlotatIndex (LocalVariables|GetFound_Index))
              (return true 0)))
          (else
            (return false (LocalVariables|GetLocal_Amount))))))
    (else
      (bind (_success__3 _index_3) (CallFunction|SearchEmptySlot))
      (if _success__3
        (bind _output_get_2 (LocalVariables|SetFound_Index _index_3))
        (Utilities|Array|SetArrayElem (Variables|Default|GetSlots) _output_get_2 (Utilities|Struct|MakeFInventorySlotStruct (LocalVariables|GetLocal_Class) 1))
        (CallFunction|UpdateSlotatIndex (LocalVariables|GetFound_Index))
        (if (> (LocalVariables|GetLocal_Amount) 1)
          (bind _rest_3 (CallFunction|AddItem (LocalVariables|GetLocal_Class) (- (LocalVariables|GetLocal_Amount) 1)))
          (return true _rest_3)
          (else
            (return true 0)))
        (else
          (return false (LocalVariables|GetLocal_Amount)))))))

(fn GetAmountatIndex
  (params (Index :type Integer))
  (return (.Amount (Utilities|Struct|BreakFInventorySlotStruct (Utilities|Array|Get(acopy) (Variables|Default|GetSlots) Index)))))

(fn ShowInventory
  (Widget|SetVisibility (Variables|Default|GetInventory_v2_Widget) "Visible")
  (Variables|Default|SetIs_Visible? true)
  (Widget|SetIsEnabled (Variables|Default|GetInventory_v2_Widget) true)
  (return))

(fn HideInventory
  (bind _inventory_v2_widget (Variables|Default|GetInventory_v2_Widget))
  (Widget|SetVisibility (Variables|Default|GetInventory_v2_Widget) "Hidden")
  (Variables|Default|SetIs_Visible? false)
  (Widget|SetIsEnabled _inventory_v2_widget false)
  (Widget|SetVisibility (Variables|/Game/Inventory_v2/Inventory_Widgets/Main_Widget.Main_Widget_C|GetThrow_Away_Widget (Variables|Default|GetMain_Widget)) "Hidden")
  (Widget|SetIsEnabled (Variables|/Game/Inventory_v2/Inventory_Widgets/Inventory_v2_Widget.Inventory_v2_Widget_C|GetSlot_Panel _inventory_v2_widget) true)
  (return))

(fn RemoveItematIndex
  (params (Index :type Integer) (Amount :type Integer))
  (bind _slots (Variables|Default|GetSlots))
  (LocalVariables|SetLocal_Index Index)
  (LocalVariables|SetLocal_Amount Amount)
  (if (and (not (CallFunction|IsSlotEmpty? (LocalVariables|GetLocal_Index))) (> (LocalVariables|GetLocal_Amount) 0))
    (if (>= (LocalVariables|GetLocal_Amount) (CallFunction|GetAmountatIndex (LocalVariables|GetLocal_Index)))
      (Utilities|Array|SetArrayElem :TargetArray (Variables|Default|GetSlots) :Index (LocalVariables|GetLocal_Index))
      (CallFunction|UpdateSlotatIndex (LocalVariables|GetLocal_Index))
      (return true)
      (else
        (Utilities|Array|SetArrayElem _slots (LocalVariables|GetLocal_Index) (Utilities|Struct|MakeFInventorySlotStruct (.itemclass (Utilities|Array|Get(acopy) _slots (LocalVariables|GetLocal_Index))) (- (.amount (Utilities|Array|Get(acopy) _slots (LocalVariables|GetLocal_Index))) (LocalVariables|GetLocal_Amount))))
        (return true)))
    (else
      (return false))))

(fn SwapSlots
  (params (Index1 :type Integer) (Index2 :type Integer))
  (bind _slots (Variables|Default|GetSlots))
  (bind _returnvalue (Utilities|Array|LastIndex _slots))
  (LocalVariables|SetLocal_Index_1 Index1)
  (LocalVariables|SetLocal_Index_2 Index2)
  (if (or (> (LocalVariables|GetLocal_Index_1) _returnvalue) (> (LocalVariables|GetLocal_Index_2) _returnvalue))
    (return false)
    (else
      (LocalVariables|SetLocal_Slot_2 (Utilities|Array|Get(acopy) (Variables|Default|GetSlots) (LocalVariables|GetLocal_Index_2)))
      (Utilities|Array|SetArrayElem (Variables|Default|GetSlots) (LocalVariables|GetLocal_Index_2) (Utilities|Array|Get(acopy) (Variables|Default|GetSlots) (LocalVariables|GetLocal_Index_1)))
      (Utilities|Array|SetArrayElem (Variables|Default|GetSlots) (LocalVariables|GetLocal_Index_1) (LocalVariables|GetLocal_Slot_2))
      (CallFunction|UpdateSlotatIndex (LocalVariables|GetLocal_Index_1))
      (CallFunction|UpdateSlotatIndex (LocalVariables|GetLocal_Index_2))
      (return true))))

(fn SplitStack
  (params (Stack_Index :type Integer) (Amount :type Integer))
  (bind _slots (Variables|Default|GetSlots))
  (LocalVariables|SetLocal_Stack_Index Stack_Index)
  (LocalVariables|SetLocal_Amount Amount)
  (if (CallFunction|IsSlotEmpty? (LocalVariables|GetLocal_Stack_Index))
    (return false)
    (elif (and (.CanBeStacked (Utilities|Struct|BreakFItemStruct (.Item_Info (CallFunction|GetItemInfoatIndex (LocalVariables|GetLocal_Stack_Index))))) (> (.Amount (CallFunction|GetItemInfoatIndex (LocalVariables|GetLocal_Stack_Index))) (LocalVariables|GetLocal_Amount)))
      (bind (_success_ _index) (CallFunction|SearchEmptySlot))
      (if _success_
        (LocalVariables|SetLocal_Found_Index _index)
        (Utilities|Array|SetArrayElem _slots (LocalVariables|GetLocal_Stack_Index) (Utilities|Struct|MakeFInventorySlotStruct (.itemclass (Utilities|Array|Get(acopy) _slots (LocalVariables|GetLocal_Stack_Index))) (- (.amount (Utilities|Array|Get(acopy) _slots (LocalVariables|GetLocal_Stack_Index))) (LocalVariables|GetLocal_Amount))))
        (Utilities|Array|SetArrayElem (Variables|Default|GetSlots) (LocalVariables|GetLocal_Found_Index) (Utilities|Struct|MakeFInventorySlotStruct (.itemclass (Utilities|Array|Get(acopy) _slots (LocalVariables|GetLocal_Stack_Index))) (LocalVariables|GetLocal_Amount)))
        (CallFunction|UpdateSlotatIndex (LocalVariables|GetLocal_Stack_Index))
        (CallFunction|UpdateSlotatIndex (LocalVariables|GetLocal_Found_Index))
        (return true)
        (else
          (return false)))
      (else
        (return false)))))

(fn AddtoIndex
  (params (From_Index :type Integer) (To_Index :type Integer))
  (LocalVariables|SetLocal_From_Index From_Index)
  (LocalVariables|SetLocal_To_Index To_Index)
  (if (Math|Boolean|ANDBoolean (== (.ItemClass (Utilities|Struct|BreakFInventorySlotStruct (Utilities|Array|Get(acopy) (Variables|Default|GetSlots) (LocalVariables|GetLocal_From_Index)))) (.ItemClass (Utilities|Struct|BreakFInventorySlotStruct (Utilities|Array|Get(acopy) (Variables|Default|GetSlots) (LocalVariables|GetLocal_To_Index))))) (< (Variables|Default|GetMax_Stack_Size) (.Amount (Utilities|Struct|BreakFInventorySlotStruct (Utilities|Array|Get(acopy) (Variables|Default|GetSlots) (LocalVariables|GetLocal_To_Index))))) (.CanBeStacked (Utilities|Struct|BreakFItemStruct (.Item_Info (CallFunction|GetItemInfoatIndex (LocalVariables|GetLocal_From_Index))))))
    (LocalVariables|SetLocal_Class (.ItemClass (Utilities|Struct|BreakFInventorySlotStruct (Utilities|Array|Get(acopy) (Variables|Default|GetSlots) (LocalVariables|GetLocal_From_Index)))))
    (if (>= (- (Variables|Default|GetMax_Stack_Size) (CallFunction|GetAmountatIndex (LocalVariables|GetLocal_To_Index))) (CallFunction|GetAmountatIndex (LocalVariables|GetLocal_From_Index)))
      (Utilities|Array|SetArrayElem (Variables|Default|GetSlots) (LocalVariables|GetLocal_To_Index) (Utilities|Struct|MakeFInventorySlotStruct (LocalVariables|GetLocal_Class) (+ (CallFunction|GetAmountatIndex (LocalVariables|GetLocal_To_Index)) (CallFunction|GetAmountatIndex (LocalVariables|GetLocal_From_Index)))))
      (Utilities|Array|SetArrayElem (Variables|Default|GetSlots) (LocalVariables|GetLocal_From_Index) (Utilities|Struct|MakeFInventorySlotStruct 0 0))
      (else
        (Utilities|Array|SetArrayElem (Variables|Default|GetSlots) (LocalVariables|GetLocal_From_Index) (Utilities|Struct|MakeFInventorySlotStruct (LocalVariables|GetLocal_Class) (- (CallFunction|GetAmountatIndex (LocalVariables|GetLocal_From_Index)) (- (Variables|Default|GetMax_Stack_Size) (CallFunction|GetAmountatIndex (LocalVariables|GetLocal_To_Index))))))
        (Utilities|Array|SetArrayElem (Variables|Default|GetSlots) (LocalVariables|GetLocal_To_Index) (Utilities|Struct|MakeFInventorySlotStruct (LocalVariables|GetLocal_Class) (Variables|Default|GetMax_Stack_Size)))))
    (CallFunction|UpdateSlotatIndex (LocalVariables|GetLocal_From_Index))
    (CallFunction|UpdateSlotatIndex (LocalVariables|GetLocal_To_Index))
    (return true)
    (else
      (return false))))

(fn SplitStacktoIndex
  (params (From_Index :type Integer) (To_Index :type Integer) (Amount :type Integer))
  (LocalVariables|SetLocal_From_Index From_Index)
  (LocalVariables|SetLocal_To_Index To_Index)
  (LocalVariables|SetLocal_Amount Amount)
  (if (Math|Boolean|ANDBoolean (CallFunction|IsSlotEmpty? (LocalVariables|GetLocal_To_Index)) (not (CallFunction|IsSlotEmpty? (LocalVariables|GetLocal_From_Index))) (.CanBeStacked (Utilities|Struct|BreakFItemStruct (.Item_Info (CallFunction|GetItemInfoatIndex (LocalVariables|GetLocal_To_Index))))) (> (.Amount (CallFunction|GetItemInfoatIndex (LocalVariables|GetLocal_To_Index))) 1) (> (.Amount (CallFunction|GetItemInfoatIndex (LocalVariables|GetLocal_To_Index))) (LocalVariables|GetLocal_Amount)))
    (LocalVariables|SetLocal_Class (.ItemClass (Utilities|Struct|BreakFInventorySlotStruct (Utilities|Array|Get(acopy) (Variables|Default|GetSlots) (LocalVariables|GetLocal_From_Index)))))
    (Utilities|Array|SetArrayElem (Variables|Default|GetSlots) (LocalVariables|GetLocal_From_Index) (Utilities|Struct|MakeFInventorySlotStruct (LocalVariables|GetLocal_Class) (- (.Amount (Utilities|Struct|BreakFInventorySlotStruct (Utilities|Array|Get(acopy) (Variables|Default|GetSlots) (LocalVariables|GetLocal_From_Index)))) (LocalVariables|GetLocal_Amount))))
    (Utilities|Array|SetArrayElem (Variables|Default|GetSlots) (LocalVariables|GetLocal_To_Index) (Utilities|Struct|MakeFInventorySlotStruct (LocalVariables|GetLocal_Class) (LocalVariables|GetLocal_Amount)))
    (CallFunction|UpdateSlotatIndex (LocalVariables|GetLocal_From_Index))
    (CallFunction|UpdateSlotatIndex (LocalVariables|GetLocal_To_Index))
    (return true)
    (else
      (return false))))

(fn ListMaker
  (params (Index :type Integer))
  (bind _item_info (CallFunction|GetItemInfoatIndex Index))
  (bind (_name _itemtype _description) (Utilities|Struct|BreakFItemStruct _item_info))
  (if (Utilities|Enum|Equal(Enum) _itemtype "Weapon")
    (Utilities|Map|Add (Variables|Default|GetWeapon_List) (Variables|Default|GetWeapon_Index) _description)
    (Math|Integer|IncrementInt (Variables|Default|GetWeapon_Index))
    (else
      (Utilities|Map|Add (Variables|Default|GetItem_List) (Variables|Default|GetItem_Index) _description)
      (Math|Integer|IncrementInt (Variables|Default|GetItem_Index)))))
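; Inventory actor that stores items in a fixed number of slots, each holding an item class and an amount.
; BeginPlay sizes the Slots array, and a slot counts as empty when its item class is invalid.
; Query functions check whether a slot is empty, return its amount and item info read from class defaults, or find the first empty slot.
; The file contains no logic for adding or removing items.
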(event EventBeginPlay
  (Utilities|Array|Resize (Variables|Default|GetSlots) (Variables|Default|GetAmount_of_Slots)))

(event Collision|EventActorBeginOverlap
  (params (OtherActor :type Actor%20Object%20Reference)))

(event EventTick
  (params (DeltaSeconds :type Float%20%28single-precision%29)))

(fn ConstructionScript)

(fn IsSlotEmpty?
  (params (Index :type Integer))
  (return (not (Utilities|IsValidClass (.ItemClass (Utilities|Struct|BreakFInventorySlotStruct (Utilities|Array|Get(acopy) (Variables|Default|GetSlots) Index)))))))

(fn GetItemInfoatIndex
  (params (Index :type Integer))
  (bind _slots (Variables|Default|GetSlots))
  (bind _output (Utilities|Array|Get(acopy) _slots Index))
  (bind (_itemclass _amount) (Utilities|Struct|BreakFInventorySlotStruct _output))
  (if (Utilities|IsValidClass _itemclass)
    (return false (Utilities|GetClassDefaults _itemclass) _amount)
    (else
      (return true "" 0))))

(fn SearchEmptySlot
  (bind (_array_element _array_index) (Utilities|Array|ForEachLoopwithBreak (Variables|Default|GetSlots) :!label _label)
    (:LoopBody
      (if (not (Utilities|IsValidClass (.ItemClass (Utilities|Struct|BreakFInventorySlotStruct _array_element))))
        (LocalVariables|SetLocal_Bool true)
        (LocalVariables|SetLocal_Index _array_index)
        (goto _label Break)))
    (:Completed
      (return (LocalVariables|GetLocal_Bool) (LocalVariables|GetLocal_Index)))))
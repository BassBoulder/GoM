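; BP_Transition is a paired portal actor that teleports the player, or a medical zombie, between linked transitions.
; Its Hit event handles the player with a door sound, while a custom event with a hit signature handles the zombie with a teleport sound.
; Both search all transitions for matching PortalIndex and opposite Entrance flag, then move the character to that actor's Exit.
; The construction script positions Portal and Exit from configurable variables.
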(event Custom|CustomEvent
  (params (MyComp :type Primitive%20Component%20Object%20Reference) (Other :type Actor%20Object%20Reference) (OtherComp :type Primitive%20Component%20Object%20Reference) (bSelfMoved :type Boolean) (HitLocation :type Vector) (HitNormal :type Vector) (NormalImpulse :type Vector) (Hit :type Hit%20Result%20Structure%20%28by%20ref%29))
  (bind _aszbp_zombie_medical (Utilities|Casting|CastToZBP_Zombie_Medical Other))
  (Audio|PlaySound2D "/Engine/VREditor/Sounds/UI/Teleport_Committed.Teleport_Committed" 1.0 1.0 0.0 0 0)
  (if (Variables|Default|GetEntrance?)
    (bind _outactors (Actor|GetAllActorsOfClass "BP_Transition_C"))
    (bind _array_element (Utilities|Array|ForEachLoopwithBreak _outactors :!label _label)
      (:LoopBody
        (if (and (== (Variables|BP_Transition_C|GetPortal_Index _array_element) (Variables|Default|GetPortal_Index)) (not (Variables|BP_Transition_C|GetEntrance? _array_element)))
          (goto _label Break)))
      (:Completed
        (Transformation|SetActorLocation _aszbp_zombie_medical (Transformation|GetWorldLocation (Variables|BP_Transition_C|GetExit _array_element)) false false)))
    (else
      (bind _outactors_2 (Actor|GetAllActorsOfClass "BP_Transition_C"))
      (bind _array_element_2 (Utilities|Array|ForEachLoopwithBreak _outactors_2 :!label _label_2)
        (:LoopBody
          (if (and (== (Variables|BP_Transition_C|GetPortal_Index _array_element_2) (Variables|Default|GetPortal_Index)) (and (not (Variables|Default|GetEntrance?)) (Variables|BP_Transition_C|GetEntrance? _array_element_2)))
            (goto _label_2 Break)))
        (:Completed
          (Transformation|SetActorLocation _aszbp_zombie_medical (Transformation|GetWorldLocation (Variables|BP_Transition_C|GetExit _array_element_2)) false false))))))

(event Collision|EventHit
  (params (MyComp :type Primitive%20Component%20Object%20Reference) (Other :type Actor%20Object%20Reference) (OtherComp :type Primitive%20Component%20Object%20Reference) (bSelfMoved :type Boolean) (HitLocation :type Vector :default "0, 0, 0") (HitNormal :type Vector :default "0, 0, 0") (NormalImpulse :type Vector :default "0, 0, 0") (Hit :type Hit%20Result%20Structure%20%28by%20ref%29))
  (bind _aszbp_player (Utilities|Casting|CastToZBP_Player Other))
  (Audio|PlaySound2D "/Game/Assets/Audio/Sound_Effects/Open_Close_Door.Open_Close_Door" 1.0 1.0 0.0 0 0)
  (if (Variables|Default|GetEntrance?)
    (bind _outactors (Actor|GetAllActorsOfClass "BP_Transition_C"))
    (bind _array_element (Utilities|Array|ForEachLoopwithBreak _outactors :!label _label)
      (:LoopBody
        (if (and (== (Variables|BP_Transition_C|GetPortal_Index _array_element) (Variables|Default|GetPortal_Index)) (not (Variables|BP_Transition_C|GetEntrance? _array_element)))
          (goto _label Break)))
      (:Completed
        (Transformation|SetActorLocation _aszbp_player (Transformation|GetWorldLocation (Variables|BP_Transition_C|GetExit _array_element)) false false)))
    (else
      (bind _outactors_2 (Actor|GetAllActorsOfClass "BP_Transition_C"))
      (bind _array_element_2 (Utilities|Array|ForEachLoopwithBreak _outactors_2 :!label _label_2)
        (:LoopBody
          (if (and (== (Variables|BP_Transition_C|GetPortal_Index _array_element_2) (Variables|Default|GetPortal_Index)) (and (not (Variables|Default|GetEntrance?)) (Variables|BP_Transition_C|GetEntrance? _array_element_2)))
            (goto _label_2 Break)))
        (:Completed
          (Transformation|SetActorLocation _aszbp_player (Transformation|GetWorldLocation (Variables|BP_Transition_C|GetExit _array_element_2)) false false))))))

(fn ConstructionScript
  ;[1 1 1] Set Portal & Exit Location
  (Transformation|SetRelativeTransform (Variables|Default|GetPortal) (Variables|Default|GetPortal_Transform) false false)
  (Transformation|SetRelativeLocation (Variables|Default|GetExit) (Variables|Default|GetExit_Location) false false))
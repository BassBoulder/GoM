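; Medical split-head zombie NPC that hunts the player and bites on contact.
; AI perception writes sensed ZBP_Player targets to the Blackboard for its AI.
; Capsule hits apply bite damage, infection and stress, while overlapping bullets are destroyed and refresh the health bar.
; AnyDamage drains health until death, which removes the capsule, flags the Blackboard, and destroys the actor after a delay, with sound cues throughout.
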(event OnPerceptionUpdated(AIPerception)
  (params (UpdatedActors :type Array%20of%20Actor%20Object%20References))
  (bind _returnvalue (AI|GetBlackboard 0))
  (for _array_element UpdatedActors
    (bind _info (Class|AIPerceptionComponent|GetActorsPerception (Variables|Default|GetAIPerception) _array_element))
    (bind _aszbp_player (Utilities|Casting|CastToZBP_Player (.Target (Utilities|Struct|BreakActorPerceptionBlueprintInfo _info))))
    (Utilities|IsValid _aszbp_player
      (:Is%20Valid
        (for _array_element_2 (.LastSensedStimuli (Utilities|Struct|BreakActorPerceptionBlueprintInfo _info))
          (if (.bSuccessfullySensed (Utilities|Struct|BreakAIStimulus _array_element_2))
            (AI|Components|Blackboard|SetValueasBool _returnvalue (Utilities|Name|MakeLiteralName "Enemy_Spotted") true)
            (AI|Components|Blackboard|SetValueasObject _returnvalue (Utilities|Name|MakeLiteralName "Enemy_Reference") (.Target (Utilities|Struct|BreakActorPerceptionBlueprintInfo _info)))
            (Variables|Default|SetIn_Range true)
            (Audio|PlaySoundatLocation "/Game/Assets/Audio/Sound_Effects/Zombie_Throat_Que.Zombie_Throat_Que" (Transformation|GetActorLocation self) "0, 0, 0" 1.0 1.0 0.0 0 0 0 0)))))))

(event OnComponentBeginOverlap(CapsuleComponent)
  (params (OverlappedComponent :type Primitive%20Component%20Object%20Reference) (OtherActor :type Actor%20Object%20Reference) (OtherComp :type Primitive%20Component%20Object%20Reference) (OtherBodyIndex :type Integer) (bFromSweep :type Boolean) (SweepResult :type Hit%20Result%20Structure%20%28by%20ref%29))
  (bind _asbp_projectile_bullet (Utilities|Casting|CastToBP_Projectile_Bullet OtherActor))
  (Utilities|IsValid _asbp_projectile_bullet
    (:Is%20Valid
      (Actor|DestroyActor _asbp_projectile_bullet)
      (CallFunction|UpdateHealthBar))))

(event OnComponentHit(CapsuleComponent)
  (params (HitComponent :type Primitive%20Component%20Object%20Reference) (OtherActor :type Actor%20Object%20Reference) (OtherComp :type Primitive%20Component%20Object%20Reference) (NormalImpulse :type Vector :default "0, 0, 0") (Hit :type Hit%20Result%20Structure%20%28by%20ref%29))
  (bind _self self)
  (if (not (Variables|Default|GetIs_Dead?))
    (bind _aszbp_player (Utilities|Casting|CastToZBP_Player OtherActor))
    (Utilities|IsValid _aszbp_player
      (:Is%20Valid
        (Game|Damage|ApplyDamage _aszbp_player (Variables|Default|GetBite) 0 _self "/Game/Blueprints/Bite_DT.Bite_DT_C")
        (Default|Infection _aszbp_player (Variables|Default|GetInfection_Value) 0 _self)
        (Default|Stress _aszbp_player (Variables|Default|GetStress_Value) 0 _self)))))

(event Custom|CustomEvent
  (params (Movement_Speed :type Float%20%28double-precision%29))
  (bind _output_get (Variables|Default|SetMovement_Speed Movement_Speed))
  (Variables|/Script/Engine.CharacterMovementComponent|SetMaxWalkSpeed (Variables|Character|GetCharacterMovement) _output_get))

(event EventBeginPlay
  (Variables|Default|SetStyle_Randomiser_Value (Math|Random|RandomIntegerinRange 0 4))
  (CallFunction|NPCSpeed (Variables|Default|GetMovement_Speed))
  (AddComponent|AddBlackboardComponent))

(event Collision|EventActorBeginOverlap
  (params (OtherActor :type Actor%20Object%20Reference))
  (|CallParentFunction OtherActor) ; This node is disabled and will not be called.\nDrag off pins to build functionality.
)

(event EventDestroyed
  (Audio|PlaySoundatLocation "/Game/Assets/Audio/Sound_Effects/Zombie_Moan_Que.Zombie_Moan_Que" (Transformation|GetActorLocation self) "0, 0, 0" 1.0 1.0 0.0 0 0 0 0))

(event EventTick
  (params (DeltaSeconds :type Float%20%28single-precision%29))
  (CallFunction|UpdateHealthBar)
  (if (Utilities|Operators|NotEqual(!=) :A (Transformation|GetVelocity))
    (Audio|PlaySoundatLocation "/Game/Assets/Audio/Sound_Effects/Walk_Shuffle_Que.Walk_Shuffle_Que" (Transformation|GetActorLocation self) "0, 0, 0" 1.0 1.0 0.0 0 0 0 0)))

(event Game|Damage|EventAnyDamage
  (params (Damage :type Float%20%28single-precision%29) (DamageType :type Damage%20Type%20Object%20Reference) (InstigatedBy :type Controller%20Object%20Reference) (DamageCauser :type Actor%20Object%20Reference))
  (bind _self self)
  (bind _returnvalue (Transformation|GetActorLocation _self))
  ;[1 1 1] Damage System
  (if (not (Variables|Default|GetIs_Dead?))
    (bind _output_get (Variables|Default|SetCurrent_Health_NPC (Math|Float|Clamp(Float) (- (Variables|Default|GetCurrent_Health_NPC) Damage) 0.0 (Variables|Default|GetMax_Health_NPC))))
    (if (== _output_get 0.0)
      (Audio|PlaySoundatLocation "/Game/Assets/Audio/Sound_Effects/Zombie_Moan_Que.Zombie_Moan_Que" _returnvalue "0, 0, 0" 1.0 1.0 0.0 0 0 0 0)
      (Variables|Default|SetIs_Dead? true)
      (Components|DestroyComponent (Variables|Default|GetCapsuleComponent))
      (AI|Components|Blackboard|SetValueasBool (AI|GetBlackboard 0) (Utilities|Name|MakeLiteralName "Is_dead?") true)
      (Utilities|FlowControl|Delay 6.5)
      (Actor|DestroyActor)
      (else
        (Audio|PlaySoundatLocation "/Game/Assets/Audio/Sound_Effects/Zombie_Injured_Que.Zombie_Injured_Que" _returnvalue "0, 0, 0" 1.0 1.0 0.0 0 0 0 0)))))

(fn ConstructionScript
  (|CallParentFunction))
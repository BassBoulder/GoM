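; Large red shelf container that the player interacts with to view its inventory.
; Interacting passes the shelf's InventorySystem to the player controller's HUD through ShowContainer.
; The HUD's InventoryOpen flag then selects the open or closed sprite, both assigned on BeginPlay.
; LookAt returns an empty string.
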(event EventBeginPlay
  (Variables|Default|SetOpen_Sprite "/Game/Assets/Items/Sprites/Item_Shelf_Open_Diffuse_Sprite_0.Item_Shelf_Open_Diffuse_Sprite_0")
  (Variables|Default|SetClose_Sprite "/Game/Assets/Items/Sprites/Item_Shelf_Sprite_0.Item_Shelf_Sprite_0"))

(event Collision|EventActorBeginOverlap
  (params (OtherActor :type Actor%20Object%20Reference)))

(event EventTick
  (params (DeltaSeconds :type Float%20%28single-precision%29)))

(event EventInteractwith
  (params (PlayerCharacter :type ZBP%20Player%20Object%20Reference))
  (bind _shelf (Variables|Default|GetShelf))
  (bind _asmy_player_controller (Utilities|Casting|CastToMy_Player_Controller (Game|GetPlayerController 0)))
  (Default|ShowContainer (Variables|/Game/Blueprints/Controllers/My_Player_Controller.My_Player_Controller_C|GetHUD _asmy_player_controller) (Variables|Default|GetInventory_System))
  (if (Variables|/Game/Inventory/Player_HUD_Widget.Player_HUD_Widget_C|GetInventory_Open (Variables|/Game/Blueprints/Controllers/My_Player_Controller.My_Player_Controller_C|GetHUD _asmy_player_controller))
    (Rendering|Components|Sprite|SetSprite _shelf (Variables|Default|GetOpen_Sprite))
    (else
      (Rendering|Components|Sprite|SetSprite _shelf (Variables|Default|GetClose_Sprite)))))

(fn ConstructionScript)

(fn Lookat
  (return ""))
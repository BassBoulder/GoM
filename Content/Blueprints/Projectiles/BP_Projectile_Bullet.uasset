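; Bullet projectile that damages medical zombies on impact, using the player's current weapon stats.
; BeginPlay caches player 0 as ZBP_Player and sets a short lifespan.
; A Sphere hit applies damage only to ZBP_Zombie_Medical, reading amount and damage type from the player at impact, then destroys the bullet whatever it struck.
; The casing hit event is empty, and some leftover nodes are unconnected.
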(event OnComponentHit(Bullet_Casing)
  (params (HitComponent :type Primitive%20Component%20Object%20Reference) (OtherActor :type Actor%20Object%20Reference) (OtherComp :type Primitive%20Component%20Object%20Reference) (NormalImpulse :type Vector :default "0, 0, 0") (Hit :type Hit%20Result%20Structure%20%28by%20ref%29)))

(event OnComponentHit(Sphere)
  (params (HitComponent :type Primitive%20Component%20Object%20Reference) (OtherActor :type Actor%20Object%20Reference) (OtherComp :type Primitive%20Component%20Object%20Reference) (NormalImpulse :type Vector :default "0, 0, 0") (Hit :type Hit%20Result%20Structure%20%28by%20ref%29))
  (bind _aszbp_zombie_medical (Utilities|Casting|CastToZBP_Zombie_Medical OtherActor)
    (:then
      (Game|Damage|ApplyDamage _aszbp_zombie_medical (Variables|/Game/Blueprints/ZBP_Player.ZBP_Player_C|GetWeapon_Damage (stale EventBeginPlay _aszbp_player)) 0 0 (Variables|/Game/Blueprints/ZBP_Player.ZBP_Player_C|GetAmmo_Type (stale EventBeginPlay _aszbp_player))))
    (:CastFailed
      _))
  (Actor|DestroyActor))

(event EventBeginPlay
  (bind _aszbp_player (Utilities|Casting|CastToZBP_Player (Game|GetPlayerCharacter 0)))
  (Actor|SetLifeSpan 5.0))

(event Collision|EventActorBeginOverlap
  (params (OtherActor :type Actor%20Object%20Reference)))

(event EventTick
  (params (DeltaSeconds :type Float%20%28single-precision%29)))

(fn ConstructionScript)
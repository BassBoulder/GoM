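; Split-head zombie Blueprint that detects the player through AI perception.
; On perception updates it filters for ZBP_Player and, for each successfully sensed stimulus, sets the spotted flag and target reference in the Blackboard, sets InRange and plays a moan at the world origin.
; Nothing here clears detection when sensing is lost, and the node writing the enemy's location to the Blackboard is unconnected.
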(event OnPerceptionUpdated(AIPerception)
  (params (UpdatedActors :type Array%20of%20Actor%20Object%20References))
  (bind _returnvalue (AI|GetBlackboard 0))
  (for _array_element UpdatedActors
    (bind _info (Class|AIPerceptionComponent|GetActorsPerception (Variables|Default|GetAIPerception) _array_element))
    (bind _aszbp_player (Utilities|Casting|CastToZBP_Player (.Target (Utilities|Struct|BreakActorPerceptionBlueprintInfo _info))))
    (Utilities|IsValid _aszbp_player
      (:Is%20Valid
        (for _array_element_2 (.LastSensedStimuli (Utilities|Struct|BreakActorPerceptionBlueprintInfo _info))
          (if (.bSuccessfullySensed (Utilities|Struct|BreakAIStimulus _array_element_2))
            (AI|Components|Blackboard|SetValueasBool _returnvalue (Utilities|Name|MakeLiteralName "Enemy_Spotted") true)
            (AI|Components|Blackboard|SetValueasObject _returnvalue (Utilities|Name|MakeLiteralName "Enemy_Reference") (.Target (Utilities|Struct|BreakActorPerceptionBlueprintInfo _info)))
            (Variables|Default|SetIn_Range true)
            (Audio|PlaySoundatLocation "/Game/Assets/Audio/Sound_Effects/Zombie_Split_Head_Moan_1_Que.Zombie_Split_Head_Moan_1_Que" "0, 0, 0" "0, 0, 0" 1.0 1.0 0.0 0 0 0 0)))))))

(event EventBeginPlay
  (|CallParentFunction) ; This node is disabled and will not be called.\nDrag off pins to build functionality.
)

(event Collision|EventActorBeginOverlap
  (params (OtherActor :type Actor%20Object%20Reference))
  (|CallParentFunction OtherActor) ; This node is disabled and will not be called.\nDrag off pins to build functionality.
)

(event EventTick
  (params (DeltaSeconds :type Float%20%28single-precision%29))
  (|CallParentFunction DeltaSeconds) ; This node is disabled and will not be called.\nDrag off pins to build functionality.
)

(fn ConstructionScript
  (|CallParentFunction))